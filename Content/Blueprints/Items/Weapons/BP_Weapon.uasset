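; Weapon Blueprint that breaks and scatters Chaos destructible objects at a supplied location.
; CreateFields uses its Field System to apply a spherical external cluster strain, then a radial linear force centred on that location.
; Nothing in this graph calls CreateFields; overlap, BeginPlay and Tick events are empty.
; Leftover movement and box-trace debug nodes are disconnected and never run.
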(event OnComponentBeginOverlap(WeaponBox)
  (params (OverlappedComponent :type Primitive%20Component%20Object%20Reference) (OtherActor :type Actor%20Object%20Reference) (OtherComp :type Primitive%20Component%20Object%20Reference) (OtherBodyIndex :type Integer) (bFromSweep :type Boolean) (SweepResult :type Hit%20Result%20Structure%20%28by%20ref%29)))

(event EventBeginPlay)

(event Collision|EventActorBeginOverlap
  (params (OtherActor :type Actor%20Object%20Reference)))

(event EventTick
  (params (DeltaSeconds :type Float%20%28single-precision%29)))

(event EventCreateFields
  (params (FieldLocation :type Vector%20%28by%20ref%29 :default "0, 0, 0"))
  (bind _fieldsystem (Variables|Default|GetFieldSystem))
  (Class|FieldSystemComponent|ApplyPhysicsField _fieldsystem true "Field_ExternalClusterStrain" 0 (Field|SetRadialFalloff (Variables|Default|GetRadialFalloff) 1e+06 0.8 1.0 0.0 2e+02 FieldLocation "Field_FallOff_None"))
  (Class|FieldSystemComponent|ApplyPhysicsField _fieldsystem true "Field_LinearForce" (Variables|Default|GetFieldSystemMetaDataFilter) (Field|SetRadialVector (Variables|Default|GetRadialVector) 1.5e+06 FieldLocation)))

(fn ConstructionScript)